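; Wall actor that orients and places itself on one side of a cell, using side flags.
; On BeginPlay, TopOrBottom yaws it 90 degrees for top or bottom walls, then Positioning teleports it 100 units from the cell's location.
; Left and right offset along X, top and bottom along Y.
; The BeginPlay call to Positioning passes no cell reference.
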(event `self.ReceiveBeginPlay`
  (`self.TopOrBottom`)
  (`self.Positioning` null))

(fn `Positioning`
  (params (CellInput :type "/Game/Blueprints/BP_Cell Object Reference"))
  (bind (_returnvalue_x _returnvalue_y _returnvalue_z) (`KismetMathLibrary.BreakVector` (`self.K2_GetActorLocation` CellInput)))
  (`|ExecutionSequence`
    (:`then_0`
      (if (`self.IsLeft`)
        (`self.K2_SetActorLocation` (`KismetMathLibrary.MakeVector` (+ _returnvalue_x -100.0) _returnvalue_y _returnvalue_z) false true)
        (return)))
    (:`then_1`
      (if (`self.IsRight`)
        (`self.K2_SetActorLocation` (`KismetMathLibrary.MakeVector` (+ _returnvalue_x 100.0) _returnvalue_y _returnvalue_z) false true)
        (return)))
    (:`then_2`
      (if (`self.IsTop`)
        (`self.K2_SetActorLocation` (`KismetMathLibrary.MakeVector` _returnvalue_x (+ _returnvalue_y 100.0) _returnvalue_z) false true)
        (return)))
    (:`then_3`
      (if (`self.IsBottom`)
        (`self.K2_SetActorLocation` (`KismetMathLibrary.MakeVector` _returnvalue_x (+ _returnvalue_y -100.0) _returnvalue_z) false true)
        (return)))))

(fn `TopOrBottom`
  (if (`self.IsTopOrBottom`)
    (`self.K2_SetActorRotation` (struct :`Pitch` 90.0) true)
    (return)))

(fn `UserConstructionScript`)