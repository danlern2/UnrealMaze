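; BP_FullCell is a maze cell actor with four toggleable walls that opens passages to neighboring cells.
; Overlap functions find neighbors by bounds and per side, but are not called within this file.
; After a short BeginPlay delay, it gathers unvisited neighbors, and RecurseBreak clears shared wall flags with a random pick; its recursive call is disconnected.
; Tick applies the flags to wall visibility and collision every frame.
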(event `self.ReceiveBeginPlay`
  (`KismetSystemLibrary.Delay` 0.2)
  (`self.BuildToVisit`)
  (`self.RecurseBreak`))

(event `self.ReceiveTick`
  (params (DeltaSeconds :type "Float (single-precision)"))
  (`self.UpdateWalls`))

(fn `BuildToVisit`
  (for _array_element (`self.AdjacentCells`)
    (if (and (== false (`/Game/Blueprints/BP_FullCell.Visited?` _array_element)) (!= _array_element null))
      (bind _output_get (set `self.ToVisitedAdjacent` (`self.ToVisitedAdjacent`)))
      (`KismetArrayLibrary.Array_Add` _output_get _array_element))))

(fn `Find Adjacent Cells`
  (bind _returnvalue (`GameplayStatics.GetObjectClass` self))
  (for _array_element (`PrimitiveComponent.GetOverlappingActors` (`self.CollisionBoundsRightLeft`) _returnvalue)
    (bind _asbp_full_cell (cast `/Game/Blueprints/BP_FullCell` _array_element))
    (if (!= self _asbp_full_cell)
      (`KismetArrayLibrary.Array_AddUnique` (`self.AdjacentCells`) _asbp_full_cell)))
  (for _array_element_2 (`PrimitiveComponent.GetOverlappingActors` (`self.CollisionBoundsFrontBack`) _returnvalue)
    (bind _asbp_full_cell_2 (cast `/Game/Blueprints/BP_FullCell` _array_element_2))
    (if (!= self _asbp_full_cell_2)
      (`KismetArrayLibrary.Array_AddUnique` (`self.AdjacentCells`) _asbp_full_cell_2))))

(fn `HideWall`
  (params (RightWall :type "Boolean (by ref)") (LeftWall :type "Boolean (by ref)") (BackWall :type "Boolean (by ref)") (FrontWall :type "Boolean (by ref)"))
  (if true
    _))

(fn `RecurseBreak`
  (bind _tovisitedadjacent (`self.ToVisitedAdjacent`))
  (bind _returnvalue (`KismetArrayLibrary.Array_Length` _tovisitedadjacent))
  (bind (_outitem _outindex) (`KismetArrayLibrary.Array_Random` _tovisitedadjacent))
  (bind _returnvalue_2 (> _returnvalue 0))
  (set `self.Visited?` true)
  (`/Engine/EditorBlueprintResources/StandardMacros.DoOnce` false :!label _label
    (:`Completed`
      (if (> _returnvalue 0)
        (if (!= _outitem null)
          (if (`/Game/Blueprints/BP_FullCell.Visited?` _outitem)
            (`KismetArrayLibrary.Array_RemoveItem` _tovisitedadjacent _outitem)
            (if _returnvalue_2
              (goto _label :!via `Reset`)
              (else
                (return)))
            (else
              (`self.WallBreakerBetweenCells` _outitem)
              (`KismetArrayLibrary.Array_Remove` _tovisitedadjacent _outindex)
              (if _returnvalue_2
                (goto _label :!via `Reset`)
                (else
                  (return))))))
        (else
          (return))))))

(fn `SetAdjacentCells`
  (bind _leftwall (`self.LeftWall`))
  (bind _rightwall (`self.RightWall`))
  (bind _backwall (`self.BackWall`))
  (bind _frontwall (`self.FrontWall`))
  (bind _array (`|MakeArray` self :!type "Actor Object Reference"))
  (`|ExecutionSequence`
    (:`then_0`
      (bind _outcomponents (`KismetSystemLibrary.ComponentOverlapComponents` _leftwall (`SceneComponent.K2_GetComponentToWorld` _leftwall) (`|MakeArray` "ObjectTypeQuery1" :!type "EObjectTypeQuery Enum") "/Script/Engine.StaticMeshComponent" _array))
      (for _array_element _outcomponents
        (bind _asbp_full_cell (cast `/Game/Blueprints/BP_FullCell` (`ActorComponent.GetOwner` _array_element)))
        (set `self.LeftAdjacent` _asbp_full_cell)
        (break)))
    (:`then_1`
      (bind _outcomponents_2 (`KismetSystemLibrary.ComponentOverlapComponents` _rightwall (`SceneComponent.K2_GetComponentToWorld` _rightwall) (`|MakeArray` "ObjectTypeQuery1" :!type "EObjectTypeQuery Enum") "/Script/Engine.StaticMeshComponent" _array))
      (for _array_element_2 _outcomponents_2
        (bind _asbp_full_cell_2 (cast `/Game/Blueprints/BP_FullCell` (`ActorComponent.GetOwner` _array_element_2)))
        (set `self.RightAdjacent` _asbp_full_cell_2)
        (break)))
    (:`then_2`
      (bind _outcomponents_3 (`KismetSystemLibrary.ComponentOverlapComponents` _backwall (`SceneComponent.K2_GetComponentToWorld` _backwall) (`|MakeArray` "ObjectTypeQuery1" :!type "EObjectTypeQuery Enum") "/Script/Engine.StaticMeshComponent" _array))
      (for _array_element_3 _outcomponents_3
        (bind _asbp_full_cell_3 (cast `/Game/Blueprints/BP_FullCell` (`ActorComponent.GetOwner` _array_element_3)))
        (set `self.BackAdjacent` _asbp_full_cell_3)
        (break)))
    (:`then_3`
      (bind _outcomponents_4 (`KismetSystemLibrary.ComponentOverlapComponents` _frontwall (`SceneComponent.K2_GetComponentToWorld` _frontwall) (`|MakeArray` "ObjectTypeQuery1" :!type "EObjectTypeQuery Enum") "/Script/Engine.StaticMeshComponent" _array))
      (for _array_element_4 _outcomponents_4
        (bind _asbp_full_cell_4 (cast `/Game/Blueprints/BP_FullCell` (`ActorComponent.GetOwner` _array_element_4)))
        (set `self.FrontAdjacent` _asbp_full_cell_4)
        (break)))))

(fn `UpdateWalls`
  (bind _frontwall (`self.FrontWall`))
  (bind _backwall (`self.BackWall`))
  (bind _rightwall (`self.RightWall`))
  (bind _leftwall (`self.LeftWall`))
  (`|ExecutionSequence`
    (:`then_0`
      (if (`self.HasLeftWall`)
        (`SceneComponent.SetHiddenInGame` _leftwall false false)
        (`PrimitiveComponent.SetCollisionEnabled` _leftwall "QueryAndPhysics")
        (else
          (`SceneComponent.SetHiddenInGame` _leftwall true false)
          (`PrimitiveComponent.SetCollisionEnabled` _leftwall "NoCollision"))))
    (:`then_1`
      (if (`self.HasRightWall`)
        (`SceneComponent.SetHiddenInGame` _rightwall false false)
        (`PrimitiveComponent.SetCollisionEnabled` _rightwall "QueryAndPhysics")
        (else
          (`SceneComponent.SetHiddenInGame` _rightwall true false)
          (`PrimitiveComponent.SetCollisionEnabled` _rightwall "NoCollision"))))
    (:`then_2`
      (if (`self.HasBackWall`)
        (`SceneComponent.SetHiddenInGame` _backwall false false)
        (`PrimitiveComponent.SetCollisionEnabled` _backwall "QueryAndPhysics")
        (else
          (`SceneComponent.SetHiddenInGame` _backwall true false)
          (`PrimitiveComponent.SetCollisionEnabled` _backwall "NoCollision"))))
    (:`then_3`
      (if (`self.HasFrontWall`)
        (`SceneComponent.SetHiddenInGame` _frontwall false false)
        (`PrimitiveComponent.SetCollisionEnabled` _frontwall "QueryAndPhysics")
        (else
          (`SceneComponent.SetHiddenInGame` _frontwall true false)
          (`PrimitiveComponent.SetCollisionEnabled` _frontwall "NoCollision"))))
    (:`then_4`
      (return))))

(fn `UserConstructionScript`)

(fn `WallBreakerBetweenCells`
  (params (Other :type "/Game/Blueprints/BP_FullCell Object Reference (by ref)"))
  (locals (Current1 :type "/Game/Blueprints/BP_FullCell Object Reference") (NewCurrent2 :type "/Game/Blueprints/BP_FullCell Object Reference") (CurrentReal :type "/Game/Blueprints/BP_FullCell Object Reference") (NewCurrentReal :type "/Game/Blueprints/BP_FullCell Object Reference"))
  (bind _asbp_full_cell (cast `/Game/Blueprints/BP_FullCell` Other))
  (if (== (`self.LeftAdjacent`) _asbp_full_cell)
    (set `/Game/Blueprints/BP_FullCell.HasRightWall` false _asbp_full_cell)
    (set `self.HasLeftWall` false)
    (return)
    (elif (== (`self.RightAdjacent`) _asbp_full_cell)
      (set `/Game/Blueprints/BP_FullCell.HasLeftWall` false _asbp_full_cell)
      (set `self.HasRightWall` false)
      (return)
      (elif (== (`self.BackAdjacent`) _asbp_full_cell)
        (set `/Game/Blueprints/BP_FullCell.HasFrontWall` false _asbp_full_cell)
        (set `self.HasBackWall` false)
        (return)
        (elif (== (`self.FrontAdjacent`) _asbp_full_cell)
          (set `/Game/Blueprints/BP_FullCell.HasBackWall` false _asbp_full_cell)
          (set `self.HasFrontWall` false)
          (return))))))