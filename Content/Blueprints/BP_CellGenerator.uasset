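; Maze generator actor that, on BeginPlay, spawns a grid of BP_FullCell actors sized by the row and column values in MainMenuGameInstance.
; Each cell finds its adjacent cells, then after staged delays random start and end cells are picked, filtered to fewer than three neighbours (grid edge).
; RecurseBreak on the chosen start cell kicks off recursive carving, which is implemented in BP_FullCell.
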(event `self.ReceiveBeginPlay`
  (`self.GenerateCells`)
  (`self.FindAdjacentCellsOfChildren`)
  (`KismetSystemLibrary.Delay` 1.0)
  (`|ExecutionSequence`
    (:`then_0`
      (`KismetSystemLibrary.Delay` 1.0)
      (bind _output_get (`self.ChooseStart`))
      (`self.ChooseEnd`))
    (:`then_1`
      (`KismetSystemLibrary.Delay` 1.0)
      (bind _asbp_full_cell (cast `/Game/Blueprints/BP_FullCell` _output_get))
      (`/Game/Blueprints/BP_FullCell.RecurseBreak` _asbp_full_cell))))

(event `self.ReceiveTick`
  (params (DeltaSeconds :type "Float (single-precision)")))

(fn `BreakLeftWallsTest`
  (bind _fullcellarray (`self.FullCellArray`))
  (bind _asmain_menu_game_instance (cast `/Game/Game/MainMenuGameInstance` (`GameplayStatics.GetGameInstance`)))
  (for (_array_element _array_index) _fullcellarray
    (if (== _array_index (- (`KismetArrayLibrary.Array_Length` _fullcellarray) (`/Game/Game/MainMenuGameInstance.RowVal` _asmain_menu_game_instance)))
      (break)
      (else
        (set `/Game/Blueprints/BP_FullCell.HasLeftWall` false _array_element)
        (`/Game/Blueprints/BP_FullCell.UpdateWalls` _array_element))))
  (return))

(fn `ChooseEnd`
  (returns (Output_Get :type "/Game/Blueprints/BP_FullCell Object Reference"))
  (locals (Ref :type "/Game/Blueprints/BP_FullCell Object Reference"))
  (`/Engine/EditorBlueprintResources/StandardMacros.DoOnce` false :!label _label
    (:`Completed`
      (bind _output_get (set `self.EndCell` (`KismetArrayLibrary.Array_Random` (`self.FullCellArray`))))
      (if (< (`KismetArrayLibrary.Array_Length` (`/Game/Blueprints/BP_FullCell.AdjacentCells` _output_get)) 3)
        (if (!= _output_get (`self.StartCell`))
          (return _output_get)
          (else
            (goto _label :!via `Reset`)))
        (else
          (goto _label :!via `Reset`))))))

(fn `ChooseStart`
  (returns (Output_Get :type "/Game/Blueprints/BP_FullCell Object Reference"))
  (`/Engine/EditorBlueprintResources/StandardMacros.DoOnce` false :!label _label
    (:`Completed`
      (bind _output_get (set `self.StartCell` (`KismetArrayLibrary.Array_Random` (`self.FullCellArray`))))
      (bind _returnvalue (`KismetArrayLibrary.Array_Length` (`/Game/Blueprints/BP_FullCell.AdjacentCells` _output_get)))
      (if (< _returnvalue 3)
        (`KismetSystemLibrary.PrintString` (`KismetStringLibrary.Conv_IntToString` _returnvalue))
        (return _output_get)
        (else
          (goto _label :!via `Reset`))))))

(fn `FindAdjacentCellsOfChildren`
  (for _array_element (`self.FullCellArray`)
    (`/Game/Blueprints/BP_FullCell.Find Adjacent Cells` _array_element)
    (`/Game/Blueprints/BP_FullCell.SetAdjacentCells` _array_element)))

(fn `GenerateCells`
  (bind (_returnvalue_x _returnvalue_y _returnvalue_z) (`KismetMathLibrary.BreakVector` (`self.K2_GetActorLocation` self)))
  (bind _asmain_menu_game_instance (cast `/Game/Game/MainMenuGameInstance` (`GameplayStatics.GetGameInstance`)))
  (for _index (range (`/Game/Game/MainMenuGameInstance.ColVal` _asmain_menu_game_instance))
    (for _index_2 (range (`/Game/Game/MainMenuGameInstance.RowVal` _asmain_menu_game_instance))
      (bind _returnvalue (`|SpawnActorFromClass` "/Game/Blueprints/BP_FullCell.BP_FullCell_C" (`KismetMathLibrary.MakeTransform` (`KismetMathLibrary.MakeVector` (+ (* _index 200) _returnvalue_x) (+ (* _index_2 200) _returnvalue_y) (+ _returnvalue_z 0.0))) "Undefined" "MultiplyWithRoot" null null))
      (`KismetArrayLibrary.Array_Add` (`self.FullCellArray`) _returnvalue))))

(fn `UserConstructionScript`)