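; BP_Cell is a cell actor that builds its own four boundary walls at runtime.
; On BeginPlay it caches its location and transform, spawns four BP_Wall actors flagged by side, gathers them into an array and has each position itself relative to the cell.
; Logic to destroy walls by per-side Has flags and an alternative MakeWalls spawner exist, but neither is wired to run.
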(event `self.ReceiveBeginPlay`
  (`|ExecutionSequence`
    (:`then_0`
      (set `self.CenterPoint` (`self.K2_GetActorLocation` self)))
    (:`then_1`
      (bind _output_get (set `self.CellTransform` (`self.GetTransform` self))))
    (:`then_2`
      (`/Engine/EditorBlueprintResources/StandardMacros.IsValid` self
        (:`Is Valid`
          (`self.SpawnWalls`)
          (`self.PopulateWalls`)
          (`self.RepositionWalls`))))))

(fn `CheckWalls`
  (`self.DestroyWalls`))

(fn `DestroyWalls`
  (`|ExecutionSequence`
    (:`then_0`
      (if (not (`self.HasLeftWall`))
        (`self.K2_DestroyActor` (`self.LeftWall`))))
    (:`then_1`
      (if (not (`self.HasRightWall`))
        (`self.K2_DestroyActor` (`self.RightWall`))))
    (:`then_2`
      (if (not (`self.HasBottomWall`))
        (`self.K2_DestroyActor` (`self.BottomWall`))))
    (:`then_3`
      (if (not (`self.HasTopWall`))
        (`self.K2_DestroyActor` (`self.TopWall`))))
    (:`then_4`
      (return))))

(fn `MakeWalls`
  (bind _output_get (`self.PopulateWalls`))
  (for _array_element _output_get
    (if true
      (`|SpawnActorFromClass` "/Game/Blueprints/BP_Wall.BP_Wall_C" (`KismetMathLibrary.Conv_VectorToTransform` (`self.K2_GetActorLocation` _array_element)) "Undefined" "MultiplyWithRoot" null _array_element false false false false false null))))

(fn `PopulateWalls`
  (returns (Output_Get :type "Array of /Game/Blueprints/BP_Wall Object Reference"))
  (bind _output_get (set `self.Walls` (`|MakeArray` (`self.LeftWall`) (`self.RightWall`) (`self.TopWall`) (`self.BottomWall`))))
  (return _output_get))

(fn `RepositionWalls`
  (for _array_element (`self.Walls`)
    (`/Game/Blueprints/BP_Wall.Positioning` _array_element self)))

(fn `SpawnWalls`
  (returns (NewParam :type Boolean))
  (for _index (range 4)
    (switch `int` _index
      (:`0`
        (bind _returnvalue (`|SpawnActorFromClass` "/Game/Blueprints/BP_Wall.BP_Wall_C" (`self.CellTransform`) "Undefined" "MultiplyWithRoot" null null false true false false false null))
        (set `self.LeftWall` _returnvalue))
      (:`1`
        (bind _returnvalue_2 (`|SpawnActorFromClass` "/Game/Blueprints/BP_Wall.BP_Wall_C" (`self.CellTransform`) "Undefined" "MultiplyWithRoot" null null false false true false false null))
        (set `self.RightWall` _returnvalue_2))
      (:`2`
        (bind _returnvalue_3 (`|SpawnActorFromClass` "/Game/Blueprints/BP_Wall.BP_Wall_C" (`self.CellTransform`) "Undefined" "MultiplyWithRoot" null null true false false true false null))
        (set `self.TopWall` _returnvalue_3))
      (:`3`
        (bind _returnvalue_4 (`|SpawnActorFromClass` "/Game/Blueprints/BP_Wall.BP_Wall_C" (`self.CellTransform`) "Undefined" "MultiplyWithRoot" null null true false false false true null))
        (set `self.BottomWall` _returnvalue_4))))
  (return false))

(fn `UserConstructionScript`)